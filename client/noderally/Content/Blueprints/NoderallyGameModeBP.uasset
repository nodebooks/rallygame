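; Game mode for Noderally, a car game with websocket-based player login, that sets a localhost server address on BeginPlay and disconnects on EndPlay.
; Authentication, new-player and connection events drive GUI messages and switches, leading to the lobby after login.
; The default pawn spawn override gives each CarBP the next body color from a cycling array.
; SpawnCar places cars at numbered START-tagged actors, but its eight-car event-graph chain never runs.
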(event EventBeginPlay
  ;[1 1 1] Assign Default Values for Host Address and Port
  (Variables|Default|Sethost "localhost")
  (Variables|Default|SetserverPort 8000))

(event EventHandleStartingNewPlayer
  (params (NewPlayer :type Player%20Controller%20Object%20Reference))
  (Development|PrintString "New player starting"))

(event EventOnNewPlayerSuccess
  (params (auth :type Player%20Auth%20Structure%20%28by%20ref%29))
  ;[1 1 1] On New Player Success
  (Default|DisplayAuthenticationMessage (Variables|Default|GetGUI) (Utilities|String|Append "New player '" (.username (Utilities|Struct|BreakPlayerAuth auth)) "' created."))
  ;[1 1 1] Clean up last login message after delay
  (Utilities|FlowControl|Delay 1.0)
  (Default|DisplayAuthenticationMessage (Variables|Default|GetGUI)))

(event EventEndPlay
  (params (EndPlayReason :type EEndPlayReason%20Enum :default "Destroyed"))
  ;[1 1 1] Disconnect Websocket
  (Class|NoderallyGameMode|DisconnectWebsocket))

(event EventOnNewPlayerFail
  (params (auth :type Player%20Auth%20Structure%20%28by%20ref%29))
  ;[1 1 1] On New Player Fail
  (Default|DisplayAuthenticationMessage (Variables|Default|GetGUI) (Utilities|String|Append "Failed to create new player '" (.username (Utilities|Struct|BreakPlayerAuth auth)) "'"))
  ;[1 1 1] Clean up last login message after delay
  (Utilities|FlowControl|Delay 1.0)
  (Default|DisplayAuthenticationMessage (Variables|Default|GetGUI)))

(event EventOnPlayerAuthenticationSuccess
  (params (auth :type Player%20Auth%20Structure%20%28by%20ref%29))
  ;[1 1 1] On Successful Authentication
  (Default|DisplayAuthenticationMessage (Variables|Default|GetGUI) "Authentication ok")
  (Utilities|FlowControl|Delay 0.5)
  (Default|DisplayLobby (Variables|Default|GetGUI)))

(event EventOnConnectionFailed
  (Development|PrintString "Could not connect"))

(event EventOnPlayerAuthenticationFail
  (params (auth :type Player%20Auth%20Structure%20%28by%20ref%29))
  ;[1 1 1] On Player Authentication Fail
  (Default|DisplayAuthenticationMessage (Variables|Default|GetGUI) (Utilities|String|Append "Authentication failed" (.reason (Utilities|Struct|BreakPlayerAuth auth))))
  ;[1 1 1] Clean up last login message after delay
  (Utilities|FlowControl|Delay 1.0)
  (Default|DisplayAuthenticationMessage (Variables|Default|GetGUI)))

(event EventOnConnectionEstablished
  (Development|PrintString "Client Connected")
  (Class|WidgetSwitcher|SetActiveWidgetIndex (Variables|/Game/GUI.GUI_C|GetviewSwitch (Variables|Default|GetGUI)) 1))

(fn ConstructionScript)

(fn SpawnCar
  (params (PlayerNumber :type Integer))
  (Utilities|FlowControl|Sequence
    (:then_0
      ;[1 1 1] Determine Spawn Point location according to Player Number
      (bind _outactors (Actor|GetAllActorswithTag (Utilities|String|StringToName (Utilities|String|Append "START" (Utilities|String|ToString(Integer) PlayerNumber)))))
      (LocalVariables|SetSpawnPointTransform (Transformation|GetActorTransform (Utilities|Array|Get(acopy) _outactors))))
    (:then_1
      ;[1 1 1] Spawn Car
      (bind _returnvalue (Game|SpawnActorfromClass "/Game/CarBP.CarBP_C" (LocalVariables|GetSpawnPointTransform) "AlwaysSpawn" 0 0))
      (LocalVariables|SetCar _returnvalue)
      (bind _asstatic_mesh_component (Utilities|Casting|CastToStaticMeshComponent (Variables|/Script/noderally.Car|GetMeshComponent _returnvalue)))
      (Rendering|Material|SetMaterial _asstatic_mesh_component 0 "/Game/BodyMaterial.BodyMaterial")
      (return (LocalVariables|GetCar)))))

(fn CreatePlayerAuth
  (return (Utilities|Struct|MakePlayerAuth (Variables|Default|Getusername) (Variables|Default|Getpassword))))

(fn SpawnDefaultPawnatTransform
  (params (NewPlayer :type Controller%20Object%20Reference) (SpawnTransform :type Transform%20%28by%20ref%29))
  (bind _returnvalue (Game|SpawnActorfromClass (Variables|Default|GetDefaultPawnClass) SpawnTransform "AlwaysSpawn" NewPlayer 0))
  (bind _ascar_bp (Utilities|Casting|CastToCarBP _returnvalue))
  (bind _asstatic_mesh_component (Utilities|Casting|CastToStaticMeshComponent (Variables|/Script/noderally.Car|GetMeshComponent _ascar_bp)))
  (CallFunction|AssignBodyColor _asstatic_mesh_component)
  (return _returnvalue))

(fn AssignBodyColor
  (params (Car :type Primitive%20Component%20Object%20Reference))
  (bind _bodycolors (Variables|Default|GetBodyColors))
  ;[1 1 1] Sets next body color according to index.
  (Rendering|Material|SetMaterial Car 0 (Utilities|Array|Get(acopy) _bodycolors (Math|Integer|%(Integer) (Variables|Default|GetnextPlayerColorIndex) (Utilities|Array|Length _bodycolors))))
  (Math|Integer|IncrementInt (Variables|Default|GetnextPlayerColorIndex)))